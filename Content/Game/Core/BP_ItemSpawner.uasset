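; BP_ItemSpawner is an interactable dispenser that gives an empty-handed character a new shop item.
; On Interaction, it spawns a BP_BaseShopObject at the character's ItemAttachPoint, copies ObjectToSpawn into its Data, sets its mesh and makes it the held item.
; The construction script applies ObjectToSpawn's mesh to the spawner itself, so it displays what it dispenses.
; A leftover debug print fires on each successful pickup.
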(event `self.ReceiveBeginPlay`)

(event `/Game/Game/Core/Interfaces/BPI_Interact.Interaction`
  (params (Character :type "/Game/Game/Core/Characters/BP_Character Object Reference"))
  (bind _output_get (set `self.Character` Character))
  (if (not (`/Game/Game/Core/Characters/BP_Character.IsHoldingItem?` Character))
    (`KismetSystemLibrary.PrintString` "asasas")
    (bind _returnvalue (`|SpawnActorFromClass` "/Game/Game/Core/Recipes/Ingredients/BP_BaseShopObject.BP_BaseShopObject_C" (`SceneComponent.K2_GetComponentToWorld` (`/Game/Game/Core/Characters/BP_Character.ItemAttachPoint` _output_get)) "AlwaysSpawn" "OverrideRootScale" null null))
    (bind _output_get_2 (set `self.SpawnedIngredientRef` _returnvalue))
    (bind _output_get_3 (set `/Game/Game/Core/Recipes/Ingredients/BP_BaseShopObject.Data` (`self.ObjectToSpawn`) _output_get_2))
    (`StaticMeshComponent.SetStaticMesh` (`/Game/Game/Core/BP_BasePickable.StaticMesh` _returnvalue) (`/Game/Game/Core/DataAssets/BP_DA_Ingredient.Mesh` _output_get_3))
    (`/Game/Game/Core/Characters/BP_Character.Set Held Item` _output_get (`self.SpawnedIngredientRef`))))

(fn `UserConstructionScript`
  (`StaticMeshComponent.SetStaticMesh` (`self.StaticMesh`) (`/Game/Game/Core/DataAssets/BP_DA_Ingredient.Mesh` (`self.ObjectToSpawn`))))