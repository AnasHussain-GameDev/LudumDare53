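; BP_Cauldron is a brewing station that turns dropped shop ingredients into potions.
; While a player is inside its Sphere, Interaction moves the held shop object into the cauldron, shrinks it and enables physics.
; CreatePotion gathers ingredient IDs from objects overlapping CauldronInsideSphere and matches them against the first three ingredients of each PotionsList recipe.
; A match spawns a BP_BasePotion with that recipe's data and mesh, then destroys the cauldron's contents.
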(event `/Game/Game/Core/Interfaces/BPI_Interact.CreatePotion`
  (bind _potionslist (`/Game/Game/Core/DataAssets/BP_DA_PotionsList.PotionsList` (`self.PotionsList`)))
  (bind _output_get (set `self.ObjectsIncauldron` (`PrimitiveComponent.GetOverlappingActors` (`self.CauldronInsideSphere`) "/Game/Game/Core/Recipes/Ingredients/BP_BaseShopObject.BP_BaseShopObject_C")))
  (for _array_element _output_get
    (bind _asbp_base_shop_object (cast `/Game/Game/Core/Recipes/Ingredients/BP_BaseShopObject` _array_element)
      (:`then`
        (`KismetArrayLibrary.Array_Add` (`self.IngredientsTobrew`) (`/Game/Game/Core/DataAssets/BP_DA_Ingredient.ID` (`/Game/Game/Core/Recipes/Ingredients/BP_BaseShopObject.Data` _asbp_base_shop_object)))
        (`KismetSystemLibrary.PrintString` "Create Potion Called from Cauldron")
        (if (`self.CanAcceptIngredients?`)
          (for (_array_element_2 _array_index) _potionslist
            (bind _output_get_2 (set `self.PotionTypeList` _array_element_2))
            (bind _ingredients (`/Game/Game/Core/DataAssets/BP_DA_Potion.Ingredients` _output_get_2))
            (for _ _ingredients
              (if (`KismetArrayLibrary.Array_Contains` (`self.IngredientsTobrew`) (`/Game/Game/Core/DataAssets/BP_DA_Ingredient.ID` (`|GetArrayItem` _ingredients)))
                (if (`KismetArrayLibrary.Array_Contains` (`self.IngredientsTobrew`) (`/Game/Game/Core/DataAssets/BP_DA_Ingredient.ID` (`|GetArrayItem` _ingredients 1)))
                  (if (`KismetArrayLibrary.Array_Contains` (`self.IngredientsTobrew`) (`/Game/Game/Core/DataAssets/BP_DA_Ingredient.ID` (`|GetArrayItem` _ingredients 2)))
                    (set `self.BrewedPotion` _output_get_2)
                    (`GameplayStatics.PlaySoundAtLocation` "/Engine/VREditor/Sounds/UI/Click_on_Button_Cue.Click_on_Button_Cue" (0.0 0.0 0.0) (struct) 1.0 1.0 0.0 null null null null)
                    (bind _output (`|GetArrayItem` _potionslist _array_index))
                    (`KismetSystemLibrary.PrintString` (`/Game/Game/Core/DataAssets/BP_DA_Potion.Name` _output))
                    (bind _returnvalue (`|SpawnActorFromClass` "/Game/Game/Core/Recipes/Potions/BP_BasePotion.BP_BasePotion_C" (`SceneComponent.K2_GetComponentToWorld` (`self.StaticMesh1`)) "AlwaysSpawn" "OverrideRootScale" null _output null))
                    (bind _output_get_3 (set `/Game/Game/Core/Recipes/Potions/BP_BasePotion.Data` (`self.BrewedPotion`) _returnvalue))
                    (`self.K2_SetActorLocation` _returnvalue (`SceneComponent.K2_GetComponentLocation` (`self.PotionSpawnLocation`)) false false)
                    (`StaticMeshComponent.SetStaticMesh` (`/Game/Game/Core/BP_BasePickable.StaticMesh` _returnvalue) (`/Game/Game/Core/DataAssets/BP_DA_Potion.PotionMesh` _output_get_3))
                    (for _array_element_3 (`self.ObjectsIncauldron`)
                      (`self.K2_DestroyActor` _array_element_3))
                    (`KismetArrayLibrary.Array_Clear` (`self.IngredientsTobrew`)))))))))
      (:`CastFailed`
        (`KismetSystemLibrary.PrintString` (`KismetSystemLibrary.GetDisplayName` _array_element))))))

(event `/Game/Game/Core/Interfaces/BPI_Interact.Interaction`
  (params (Character :type "/Game/Game/Core/Characters/BP_Character Object Reference"))
  (bind _helditem (`/Game/Game/Core/Characters/BP_Character.HeldItem` Character))
  (bind (_returnvalue_location _returnvalue_rotation _returnvalue_scale) (`KismetMathLibrary.BreakTransform` (`SceneComponent.K2_GetComponentToWorld` (`self.StaticMesh1`))))
  (if (`self.CanAcceptIngredients?`)
    (`/Engine/EditorBlueprintResources/StandardMacros.IsValid` _helditem
      (:`Is Valid`
        (cast `/Game/Game/Core/Recipes/Ingredients/BP_BaseShopObject` _helditem)
        ;[1 0 0] HotFix: to set held item to cauldron
        (set `/Game/Game/Core/Characters/BP_Character.IsHoldingItem?` false Character)
        (`self.K2_DetachFromActor` _helditem "KeepRelative" "KeepRelative" "KeepRelative")
        (`self.K2_SetActorTransform` _helditem (`KismetMathLibrary.MakeTransform` _returnvalue_location _returnvalue_rotation (* _returnvalue_scale 0.25)) false true)
        (`PrimitiveComponent.SetSimulatePhysics` (`/Game/Game/Core/BP_BasePickable.StaticMesh` _helditem) true)
        (set `/Game/Game/Core/Characters/BP_Character.HeldItem` null Character)))))

(event `self.Sphere.OnComponentBeginOverlap`
  (params (OverlappedComponent :type "PrimitiveComponent Object Reference") (OtherActor :type "Actor Object Reference") (OtherComp :type "PrimitiveComponent Object Reference") (OtherBodyIndex :type Integer) (bFromSweep :type Boolean) (SweepResult :type "HitResult Structure (by ref)"))
  (if (`self.ActorHasTag` OtherActor "Player")
    (set `self.CanAcceptIngredients?` true)))

(event `self.Sphere.OnComponentEndOverlap`
  (params (OverlappedComponent :type "PrimitiveComponent Object Reference") (OtherActor :type "Actor Object Reference") (OtherComp :type "PrimitiveComponent Object Reference") (OtherBodyIndex :type Integer))
  (if (`self.ActorHasTag` OtherActor "Player")
    (set `self.CanAcceptIngredients?` false)))

(fn `UserConstructionScript`)