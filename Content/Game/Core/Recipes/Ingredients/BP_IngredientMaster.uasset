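; Master ingredient actor that hands the interacting character an ingredient item.
; On Interaction, it looks up its IngredientName in the DTIngredient data table and prints the row's ingredient name.
; It spawns that row's actor class at the character's ItemAttachPoint, ignoring collisions, and snap-attaches it there.
; The source actor stays in place, and a missing row does nothing.
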(event `self.ReceiveBeginPlay`)

(event `/Game/Game/Core/Interfaces/BPI_Interact.Interaction`
  (params (Character :type "/Game/Game/Core/Characters/BP_Character Object Reference"))
  (set `self.Character` Character)
  (bind _returnvalue (`|GetDataTableRow` "/Game/Game/Core/Recipes/DTIngredient.DTIngredient" (`self.IngredientName`))
    (:`then`
      (bind (_nameofingredient _ingredientactor) (break `/Game/Game/Core/Recipes/SIngredient` _returnvalue))
      (`KismetSystemLibrary.PrintString` _nameofingredient)
      (bind _returnvalue_2 (`|SpawnActorFromClass` _ingredientactor (`SceneComponent.K2_GetComponentToWorld` (`/Game/Game/Core/Characters/BP_Character.ItemAttachPoint` Character)) "AlwaysSpawn" "OverrideRootScale" null null))
      (`self.K2_AttachToComponent` _returnvalue_2 (`/Game/Game/Core/Characters/BP_Character.ItemAttachPoint` (`self.Character`)) "None" "SnapToTarget" "SnapToTarget" "SnapToTarget" true))))

(fn `UserConstructionScript`)