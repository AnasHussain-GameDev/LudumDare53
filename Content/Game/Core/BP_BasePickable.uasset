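; BP_BasePickable is a base Blueprint for pickable items, handling what happens when the player drops a held item.
; On BeginPlay it binds to the OnDropHeldItem event of the player's BP_Character, and on Destroyed it unbinds.
; The handler acts on the item passed by the event rather than on itself, detaching its StaticMesh in world space, enabling physics and printing a debug string.
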(event `self.ReceiveBeginPlay`
  (bind _asbp_character (cast `/Game/Game/Core/Characters/BP_Character` (`GameplayStatics.GetPlayerCharacter` 0)))
  (add `/Game/Game/Core/Characters/BP_Character.OnDropHeldItem` _asbp_character (delegate `OnDropItemHeld`)))

(event `OnDropItemHeld`
  (params (NewParam :type "/Game/Game/Core/BP_BasePickable Object Reference"))
  ;[1 1 1] Getting Fired 3 times instead of 1, needs fixing. - Fixed, it was because it was applying to all of the ones that were force spawned
  (`SceneComponent.K2_DetachFromComponent` (`/Game/Game/Core/BP_BasePickable.StaticMesh` NewParam) "KeepWorld" "KeepWorld" "KeepWorld" true)
  (`PrimitiveComponent.SetSimulatePhysics` (`/Game/Game/Core/BP_BasePickable.StaticMesh` NewParam) true)
  (`KismetSystemLibrary.PrintString` "Hello"))

(event `self.ReceiveDestroyed`
  (bind _asbp_character (cast `/Game/Game/Core/Characters/BP_Character` (`GameplayStatics.GetPlayerCharacter` 0)))
  (remove `/Game/Game/Core/Characters/BP_Character.OnDropHeldItem` _asbp_character (delegate `OnDropItemHeld`)))

(fn `UserConstructionScript`)