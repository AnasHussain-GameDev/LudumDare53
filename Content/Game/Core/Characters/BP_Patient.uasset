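; BP_Patient is an AI customer with an illness that the player cures by handing over the matching potion.
; On BeginPlay it maps its illness enum to a cure data asset, labels its name tag and walks patrol points to the counter.
; Interaction compares the held potion's name to the cure, consuming it on a match.
; Cured patients, or uncured ones after a timed wait, walk out and self-destroy, with score changes only printed.
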(event `self.ReceiveBeginPlay`
  (bind _returnvalue (`|GetEnumeratorNameAsString` (`self.Illness`)))
  ;[1 1 1] Iterates through an enum and sets the cure variable  based on the enum
  (`self.GetIllnessAndCure`)
  ;[1 1 1] Prints the illness and the cure to us for testing purposes
  (`KismetSystemLibrary.PrintString` (`KismetSystemLibrary.GetDisplayName` (`self.Cure`)))
  (`KismetSystemLibrary.PrintString` _returnvalue)
  (bind _aswbp_name_tag (cast `/Game/Game/Core/Widgets/WBP_NameTag` (`WidgetComponent.GetWidget` (`self.Widget`))))
  (set `/Game/Game/Core/Widgets/WBP_NameTag.PickableName` _returnvalue _aswbp_name_tag)
  ;[1 1 1] Move to the counter and face the player
  (`|AIMoveTo` self (`|GetArrayItem` (`self.PatrolPoints`)) null
    (:`OnSuccess`
      (`|AIMoveTo` self (`|GetArrayItem` (`self.PatrolPoints`) 1) null
        (:`OnSuccess`
          (`|AIMoveTo` self (`|GetArrayItem` (`self.PatrolPoints`) 2) null
            (:`OnSuccess`
              ;;[1 1 1] Calls this in tandem with the set timer by event node in BP_PatientSpawner so the current customer leaves when the new one walks up to the counter
              (`self.K2_SetActorRotation` (`KismetMathLibrary.MakeRotator` 0.0))
              (`KismetSystemLibrary.Delay` 20.0)
              (`self.HasNotBeenCured`))))))))

(event `HasBeenCured`
  (bind _patrolpoints (`self.PatrolPoints`))
  ;[1 1 1] Patient leaving after having been cured ( I used event interaction in the blueprint interface, but we can get it to work with the table
  (`KismetSystemLibrary.PrintString` "+50 points!")
  (if (`self.IsCured?`)
    (`|AIMoveTo` self (`|GetArrayItem` _patrolpoints 3) null
      (:`OnSuccess`
        (`|AIMoveTo` self (`|GetArrayItem` _patrolpoints 4) null
          (:`OnSuccess`
            (`self.K2_DestroyActor`)))))))

(event `HasNotBeenCured`
  (bind _patrolpoints (`self.PatrolPoints`))
  ;[1 1 1] Patient leaves without being treated, granting negative points.
  (`KismetSystemLibrary.PrintString` "-50 points!")
  (if (not (`self.IsCured?`))
    (`|AIMoveTo` self (`|GetArrayItem` _patrolpoints 3) null
      (:`OnSuccess`
        (`|AIMoveTo` self (`|GetArrayItem` _patrolpoints 4) null
          (:`OnSuccess`
            (`self.K2_DestroyActor`)))))))

(event `/Game/Game/Core/Interfaces/BPI_Interact.Interaction`
  (params (Character :type "/Game/Game/Core/Characters/BP_Character Object Reference"))
  (bind _helditem (`/Game/Game/Core/Characters/BP_Character.HeldItem` Character))
  ;[1 1 1] Checks if the potion we are holding has the exact name that the illness is required to have to cure it, and if it does, sets Iscured? to true so patient can leave
  (bind _asbp_base_potion (cast `/Game/Game/Core/Recipes/Potions/BP_BasePotion` _helditem))
  (if (`KismetStringLibrary.EqualEqual_StrStr` (`/Game/Game/Core/DataAssets/BP_DA_Potion.Name` (`/Game/Game/Core/Recipes/Potions/BP_BasePotion.Data` _asbp_base_potion)) (`/Game/Game/Core/DataAssets/BP_DA_Potion.Name` (`self.Cure`)))
    (set `self.IsCured?` true)
    (`self.HasBeenCured`)
    (`self.K2_DestroyActor` _helditem)
    (set `/Game/Game/Core/Characters/BP_Character.IsHoldingItem?` false Character)))

(fn `GetIllnessAndCure`
  (if (`|EnumEquality` (`self.Illness`) "NewEnumerator0")
    (set `self.Cure` "/Game/Game/Core/DataAssets/Potions/DA_WerewolfsCure.DA_WerewolfsCure")
    (elif (`|EnumEquality` (`self.Illness`) "NewEnumerator2")
      (set `self.Cure` "/Game/Game/Core/DataAssets/Potions/DA_MinotaurMazeCure.DA_MinotaurMazeCure")
      (elif (`|EnumEquality` (`self.Illness`) "NewEnumerator3")
        (set `self.Cure` "/Game/Game/Core/DataAssets/Potions/DA_TrollsPoxCure.DA_TrollsPoxCure")
        (elif (`|EnumEquality` (`self.Illness`) "NewEnumerator1")
          (set `self.Cure` "/Game/Game/Core/DataAssets/Potions/DA_MedusasTouch.DA_MedusasTouch")
          (elif (`|EnumEquality` (`self.Illness`) "NewEnumerator4")
            (set `self.Cure` "/Game/Game/Core/DataAssets/Potions/DA_GoblinRotBalm.DA_GoblinRotBalm")
            (elif (`|EnumEquality` (`self.Illness`) "NewEnumerator6")
              (set `self.Cure` "/Game/Game/Core/DataAssets/Potions/DA_FaerieFever.DA_FaerieFever")
              (elif (`|EnumEquality` (`self.Illness`) "NewEnumerator7")
                (set `self.Cure` "/Game/Game/Core/DataAssets/Potions/DA_DragonBreathPoultice.DA_DragonBreathPoultice")
                (elif (`|EnumEquality` (`self.Illness`) "NewEnumerator5")
                  (set `self.Cure` "/Game/Game/Core/DataAssets/Potions/DA_BansheesWailCure.DA_BansheesWailCure"))))))))))

(fn `UserConstructionScript`)